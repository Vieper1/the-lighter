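; Game instance that holds and persists level progress for the game, exposed through write-save and load-save events.
; Loading reads slot "0" into a LighterSaveData object, which saving creates if missing.
; Saving overwrites the level's finish time without comparing it, then adds any missing levels to unlock with zero time.
; Each map write triggers its own async save to disk, which prints success or failure.
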(event Custom|Event_WriteSave
  (params (LevelName :type Name) (FinishTime :type Float%20%28single-precision%29) (LevelsToUnlock :type Array%20of%20Names))
  ;[1 1 1] Save
  (Utilities|SaveCurrentLevel LevelName FinishTime LevelsToUnlock))

(event Custom|Event_LoadSave
  ;[1 1 1] Load
  (Utilities|LoadSaveData))