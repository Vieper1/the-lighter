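; BrokenSpotLight is a prop that makes a spot light flicker like a faulty lamp.
; The construction script caches the light's authored intensity, and BeginPlay starts it dark.
; Tick counts down a timer and, on expiry, toggles between the cached and minimum intensity.
; Each on or off phase gets a random duration capped by its own maximum time.
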(event EventTick
  (params (DeltaSeconds :type Float%20%28single-precision%29))
  (Variables|State|SetTimeLeft (- (Variables|State|GetTimeLeft) DeltaSeconds))
  (if (< (Variables|State|GetTimeLeft) 0.0)
    (bind _output_get (Variables|Default|SetIsOn (not (Variables|Default|GetIsOn))))
    (Variables|State|SetTimeLeft (Math|Random|RandomFloatinRange 0.01 (select _output_get (Variables|Config|GetMaxONTime) (Variables|Config|GetMaxOFFTime))))
    (Rendering|Components|Light|SetIntensity (Variables|Default|GetSpotLight) (select _output_get (Variables|Config|GetInitialIntensity) (Variables|Config|GetMinIntensity)))))

(event EventBeginPlay
  (Rendering|Components|Light|SetIntensity (Variables|Default|GetSpotLight) 0.0))

(fn ConstructionScript
  (Variables|Config|SetInitialIntensity (Variables|/Script/Engine.LightComponentBase|GetIntensity (Variables|Default|GetSpotLight))))