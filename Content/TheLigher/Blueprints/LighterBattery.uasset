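; LighterBattery is the level-end pickup that sends the player on to the next level when collected.
; On pickup it detaches the PlayerBall, plays the endpoint-activated Niagara effect, triggers GM_Gameplay's pickup drama and next-level load, then destroys itself.
; Until then, a looping timer fakes a signal broadcast by adding Niagara components.
; The radial SignalUnit spawner and a slow-motion pickup branch remain in the graph but never run.
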(event Custom|Event_BroadcastSignal
  ;[1 1 1] Start fake broadcast particle
  (AddComponent|AddNiagaraComponent false))

(event Custom|OnPickedUp
  (bind _returnvalue (Transformation|GetActorTransform))
  ;[1 1 1] On Battery Picked Up
  (Class|NiagaraComponent|SetAsset (Variables|Default|GetNiagaraEmitter) "/Game/Geometry/VFX/p_endpoint_activated.p_endpoint_activated")
  (bind _asplayer_ball (Utilities|Casting|CastToPlayerBall (Game|Player|GetPlayerPawn 0)))
  (Class|TheLighterBall|DetachPlayerBall _asplayer_ball)
  (Niagara|SpawnSystematLocation "/Game/Geometry/VFX/p_endpoint_activated.p_endpoint_activated" (.location _returnvalue) (.rotation _returnvalue) (.scale _returnvalue))
  (bind _asgm_gameplay (Utilities|Casting|CastToGM_Gameplay (Game|GetGameMode)))
  (Default|EventBatteryPickupDrama _asgm_gameplay (.location _returnvalue))
  (bind _asgm_gameplay_2 (Utilities|Casting|CastToGM_Gameplay (Game|GetGameMode)))
  (Default|EventLoadNextLevel _asgm_gameplay_2)
  (Actor|DestroyActor))

(event EventBeginPlay
  (Utilities|FlowControl|Sequence
    (:then_0
      ;[1 1 1] On Battery Picked Up
      (EventDispatchers|BindEventtoEventonPickedUp (delegate Custom|OnPickedUp)))
    (:then_1
      ;[1 1 1] Start fake broadcast particle
      (Utilities|Time|SetTimerbyEvent (delegate Custom|Event_BroadcastSignal) (Variables|SignalConfig|GetSignalDelay) true (Variables|SignalConfig|GetStartDelay)))))

(fn ConstructionScript
  (|CallParentFunction))

(fn BroadcastSignalUnits
  (bind _numberofunits (Variables|SignalConfig|GetNumberOfUnits))
  (for _index (range 0 (- _numberofunits 1))
    (Game|SpawnActorfromClass (Variables|Config|GetSignalUnitClass) (Math|Transform|MakeTransform (+ (Transformation|GetActorLocation) (* (Math|Vector|GetForwardVector (Math|Rotator|MakeRotator 0.0 (+ (* (Math|Conversions|ToFloat(Integer) _index) (/ 3.6e+02 (Math|Conversions|ToFloat(Integer) _numberofunits))) 0.0) 9e+01)) (Variables|SignalConfig|GetSignalSpawnCorrection))) (Math|Rotator|MakeRotator 0.0 (+ (* (Math|Conversions|ToFloat(Integer) _index) (/ 3.6e+02 (Math|Conversions|ToFloat(Integer) _numberofunits))) 0.0) 9e+01) "0.300000,0.300000,0.300000") "AdjustIfPossibleButAlwaysSpawn" 0 0)))