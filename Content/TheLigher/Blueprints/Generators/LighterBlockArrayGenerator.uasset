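; LighterBlockArrayGenerator is a generator actor that builds a flat grid of lighter blocks as child actor components.
; Its construction script clears the block array, then adds scaled components until it holds RowCount times ColumnCount entries.
; GetCoordinates turns each index into column and row, spacing blocks evenly across Width and Height.
; Relative offsets use the actor's world-space right and up vectors, starting at the origin.
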(fn ConstructionScript
  (bind _lighterblockarray (Variables|Default|GetLighterBlockArray))
  (Utilities|Array|Clear (Variables|Default|GetLighterBlockArray))
  (while (!= (Utilities|Array|Length (Variables|Default|GetLighterBlockArray)) (* (Variables|Default|GetRowCount) (Variables|Default|GetColumnCount)))
    (bind _returnvalue (AddComponent|AddChildActorComponent false (Math|Transform|MakeTransform "0, 0, 0" "0, 0, 0" (Variables|Default|GetBlockScale))))
    (bind _returnvalue_2 (Utilities|Array|Add _lighterblockarray _returnvalue))
    (Transformation|SetRelativeLocation (Utilities|Array|Get(acopy) _lighterblockarray _returnvalue_2) (+ (* (* (/ (Transformation|GetActorUpVector) (Math|Conversions|ToFloat(Integer) (- (Variables|Default|GetRowCount) 1))) (Variables|Default|GetHeight)) (Math|Conversions|ToFloat(Integer) (.Y (CallFunction|GetCoordinates _returnvalue_2)))) (* (* (/ (Transformation|GetActorRightVector) (Math|Conversions|ToFloat(Integer) (- (Variables|Default|GetColumnCount) 1))) (Variables|Default|GetWidth)) (Math|Conversions|ToFloat(Integer) (.X (CallFunction|GetCoordinates _returnvalue_2))))) false false)))

(fn GetCoordinates
  (params (Index :type Integer))
  (return (Math|Integer|%(Integer) Index (Variables|Default|GetColumnCount)) (/ Index (Variables|Default|GetColumnCount))))