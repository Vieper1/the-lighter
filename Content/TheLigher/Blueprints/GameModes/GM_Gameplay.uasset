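; Gameplay game mode that respawns the player ball and advances to the next level.
; On BeginPlay it caches the PlayerBall pawn and records its starting location as the spawn point.
; The respawn event teleports the ball back there with zero rotation and clears the linear velocity of its physics body.
; The load event waits briefly, then opens the level named by NextLevelName.
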(event Custom|Event_RespawnPlayer
  (bind _playerball (Variables|Default|GetPlayerBall))
  ;[1 1 1] Respawn Logic
  (Utilities|IsValid _playerball
    (:Is%20Valid
      (Transformation|Teleport _playerball (Variables|State|GetSpawnLocation) "0, 0, 0")
      (Physics|SetPhysicsLinearVelocity (Variables|/Script/TheLighter.TheLighterBall|GetBall _playerball) "0, 0, 0" false "None"))))

(event Custom|Event_LoadNextLevel
  ;[1 1 1] Load Level
  (Utilities|FlowControl|Delay 1.5)
  (Game|OpenLevel(byName) (Variables|Default|GetNextLevelName)))

(event EventBeginPlay
  (bind _asplayer_ball (Utilities|Casting|CastToPlayerBall (Game|Player|GetPlayerPawn 0)))
  (bind _output_get (Variables|Default|SetPlayerBall _asplayer_ball))
  (Variables|State|SetSpawnLocation (Transformation|GetActorLocation _output_get)))

(fn ConstructionScript)